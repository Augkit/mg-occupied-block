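; Player controller that glides the controlled pawn to requested transforms and creates UI widgets for scoreboards and modals.
; MoveControlledPawnTo stores a target that Tick approaches with TInterpTo and teleporting, snapping when nearly equal; the moving flag is never cleared.
; Player scoreboards are added to and removed from a horizontal layout widget, created lazily on first use.
; Info and transition modals are created fresh, added to the viewport and returned to the caller.
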(event EventBeginPlay)

(event EventTick
  (params (DeltaSeconds :type Float%20%28single-precision%29))
  (if (Variables|Default|GetIsMovingPawn)
    (if (Class|KismetMathLibrary|NearlyEqualTransformTransform (Transformation|GetActorTransform (Pawn|GetControlledPawn)) (Variables|Default|GetPawnTargetTransform) 0.0001 0.0001 0.0001)
      (Variables|Default|SetIsMovingPawn true)
      (Transformation|SetActorTransform (Pawn|GetControlledPawn) (Variables|Default|GetPawnTargetTransform) false true)
      (else
        (Transformation|SetActorTransform (Pawn|GetControlledPawn) (Class|KismetMathLibrary|TInterpto (Transformation|GetActorTransform (Pawn|GetControlledPawn)) (Variables|Default|GetPawnTargetTransform) DeltaSeconds 5.0) false true)))))

(fn ConstructionScript)

(fn CreatePlayerScoreboard
  (Variables|Default|GetPlayerScoreboards
    (:then
      _)
    (:else
      ;[1 1 1] 懒加载
      (bind _returnvalue (UserInterface|CreateWidget "/Game/UMG/BPW_HorizontalLayout.BPW_HorizontalLayout_C" self))
      (bind _output_get (Variables|Default|SetPlayerScoreboards _returnvalue))
      (UserInterface|Viewport|AddtoViewport _output_get 0)))
  (bind _returnvalue_2 (UserInterface|CreateWidget "/Game/UMG/BPW_PlayerScoreboard.BPW_PlayerScoreboard_C" self))
  (Default|AddChild (Variables|Default|GetPlayerScoreboards) _returnvalue_2)
  (return _returnvalue_2))

(fn RemovePlayerScoreboard
  (params (Content :type Widget%20Object%20Reference))
  (Default|RemoveChild (Variables|Default|GetPlayerScoreboards) Content))

(fn MoveControlledPawnto
  (params (NewTransform :type Transform%20%28by%20ref%29))
  (Variables|Default|SetPawnTargetTransform NewTransform)
  (Variables|Default|SetIsMovingPawn true))

(fn OpenInfoModal
  (bind _returnvalue (UserInterface|CreateWidget "/Game/UMG/Modal/BPW_Modal.BPW_Modal_C" self))
  (UserInterface|Viewport|AddtoViewport _returnvalue 0)
  (return _returnvalue))

(fn OpenTransitionModal
  (bind _returnvalue (UserInterface|CreateWidget "/Game/UMG/Modal/BPW_Transition.BPW_Transition_C" self))
  (UserInterface|Viewport|AddtoViewport _returnvalue 0)
  (return _returnvalue))