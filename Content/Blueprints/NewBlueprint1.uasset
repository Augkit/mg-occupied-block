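; Test-style Blueprint that drives a tetromino on a checkerboard through a BP_CheckerboardController.
; Input actions step the piece in four directions or place it; K prints the vacancy check result, then rotates and moves the piece to the returned spot unconditionally.
; BeginPlay only yaws the actor 90 degrees.
; Controller and tetromino setup and timed-rotation logic are disconnected, and InitCheckerboard, which creates the controller and board, is never called here.
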(event Custom|CustomEvent_0
  (Class|Tetromino|Rotate90Degrees (Variables|Default|GetTetromino) -1.0)
  (Utilities|FlowControl|Delay 0.2))

(event EventBeginPlay
  (Class|Actor|AddActorWorldRotation "0,90.000000, 0"))

(event Input|ActionEvents|InputActionMoveUp
  (params (Key :type Key%20Structure))
  (:Pressed
    (Class|CheckerboardController|MoveTetrominoonBoardbyStep (Variables|Default|GetController) "(X=0.000000,Y=-1.000000)")))

(event Input|ActionEvents|InputActionMoveDown
  (params (Key :type Key%20Structure))
  (:Pressed
    (Class|CheckerboardController|MoveTetrominoonBoardbyStep (Variables|Default|GetController) "(X=0.000000,Y=1.000000)")))

(event Input|ActionEvents|InputActionMoveRight
  (params (Key :type Key%20Structure))
  (:Pressed
    (Class|CheckerboardController|MoveTetrominoonBoardbyStep (Variables|Default|GetController) "(X=1.000000,Y=0.000000)")))

(event Input|ActionEvents|InputActionMoveLeft
  (params (Key :type Key%20Structure))
  (:Pressed
    (Class|CheckerboardController|MoveTetrominoonBoardbyStep (Variables|Default|GetController) "(X=-1.000000,Y=0.000000)")))

(event Input|ActionEvents|InputActionInteractAction
  (params (Key :type Key%20Structure))
  (:Pressed
    (Class|CheckerboardController|PutTetrominotoBoard (Variables|Default|GetController))))

(event Input|KeyboardEvents|K
  (params (Key :type Key%20Structure))
  (:Pressed
    (bind (_validlocation _validdegrees _returnvalue) (Class|CheckerboardController|CheckTetrominoVacancies (Variables|Default|GetController) (Variables|Default|GetTetromino)))
    (Development|PrintString (Utilities|String|Append (Utilities|String|ToString(Vector2d) _validlocation) " " (Utilities|String|ToString(Float) _validdegrees) " " (Utilities|String|ToString(Boolean) _returnvalue)))
    (if true
      (Class|Tetromino|Rotateto (Variables|Default|GetTetromino) _validdegrees)
      (Class|CheckerboardController|MoveTetrominotoBoardLocation (Variables|Default|GetController) (Variables|Default|GetTetromino) _validlocation))))

(fn ConstructionScript)

(fn InitCheckerboard
  (Utilities|FlowControl|Sequence
    (:then_0
      (bind _returnvalue (Game|ConstructObjectfromClass "/Game/Blueprints/BP_CheckerboardController.BP_CheckerboardController_C" self))
      (Variables|Default|SetController _returnvalue))
    (:then_1
      (bind _returnvalue_2 (Game|SpawnActorfromClass "/Game/Blueprints/BP_Checkerboard.BP_Checkerboard_C" (Transformation|GetActorTransform) "Undefined" 0 0))
      (Variables|Default|SetCheckerboard _returnvalue_2))
    (:then_2
      (Class|CheckerboardController|SetCheckerboard (Variables|Default|GetController) (Variables|Default|GetCheckerboard)))))