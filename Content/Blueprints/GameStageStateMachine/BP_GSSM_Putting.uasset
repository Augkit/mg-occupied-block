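; BP_GSSM_Putting is the game stage state for placing the selected tetromino on the board.
; On entering, it moves the selected tetromino to the board and the camera to the checkerboard focus point.
; Input interface events forward to the playground to move or rotate the piece, put it down, or return to selecting.
; The state holds no placement logic, and its exit only calls the parent.
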(event EventBPIExecuteMoveUp
  (params (GamePlayerground :type BP%20Game%20Playground%20Object%20Reference) (Controller :type Checkerboard%20Controller%20Object%20Reference))
  (Default|MoveTetrominoUp GamePlayerground))

(event EventBPIExecuteMoveDown
  (params (GamePlayerground :type BP%20Game%20Playground%20Object%20Reference) (Controller :type Checkerboard%20Controller%20Object%20Reference))
  (Default|MoveTetrominoDown GamePlayerground))

(event EventBPIExecuteMoveRight
  (params (GamePlayerground :type BP%20Game%20Playground%20Object%20Reference) (Controller :type Checkerboard%20Controller%20Object%20Reference))
  (Default|MoveTetrominoRight GamePlayerground))

(event EventBPIExecuteMoveLeft
  (params (GamePlayerground :type BP%20Game%20Playground%20Object%20Reference) (Controller :type Checkerboard%20Controller%20Object%20Reference))
  (Default|MoveTetrominoLeft GamePlayerground))

(event EventBPIExecuteInteract
  (params (GamePlayerground :type BP%20Game%20Playground%20Object%20Reference) (Controller :type Checkerboard%20Controller%20Object%20Reference))
  (Default|PutTetrominotoBoard GamePlayerground))

(event EventBPIExecuteBack
  (params (GamePlayerground :type BP%20Game%20Playground%20Object%20Reference) (Controller :type Checkerboard%20Controller%20Object%20Reference))
  (Default|BacktoSelecting GamePlayerground))

(event EventBPIExexuteRotate
  (params (GamePlayerground :type BP%20Game%20Playground%20Object%20Reference) (Controller :type Checkerboard%20Controller%20Object%20Reference))
  (Default|RotateTetromino GamePlayerground))

(fn OnBeginGameStage
  (params (Playground :type BP%20Game%20Playground%20Object%20Reference) (PrevStage :type Enum_GameStage%20Enum :default "NewEnumerator7"))
  (|CallParentFunction Playground PrevStage)
  (Default|MoveSelectedTetrominotoBoard Playground)
  (Default|MoveCameratoFocusPoint Playground (Variables|/Game/Blueprints/BP_GamePlayground.BP_GamePlayground_C|GetFocusCheckerboardTransform Playground)))

(fn OnEndGameStage
  (params (Playground :type BP%20Game%20Playground%20Object%20Reference) (NextStage :type Enum_GameStage%20Enum :default "NewEnumerator7"))
  (|CallParentFunction Playground NextStage))