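; Game-begin stage of the game stage state machine, which sets up a new game on the playground.
; On entry it creates and assigns a checkerboard controller, initializes the player, shows a "游戏开始" (Game Start) info modal and resets the round counter to zero.
; An interact event closes the modal, if valid, and switches the playground to another stage.
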(event EventBPIExecuteInteract
  (params (GamePlayerground :type BP%20Game%20Playground%20Object%20Reference) (Controller :type Checkerboard%20Controller%20Object%20Reference))
  (bind _modal_widget (Variables|Default|GetModal%20Widget)
    (:then
      (Class|ModalWidget|Close _modal_widget)
      (Default|SetGameStage GamePlayerground "NewEnumerator5"))
    (:else)))

(fn OnBeginGameStage
  (params (Playground :type BP%20Game%20Playground%20Object%20Reference) (PrevStage :type Enum_GameStage%20Enum :default "NewEnumerator7"))
  (|CallParentFunction Playground PrevStage)
  (Utilities|FlowControl|Sequence
    (:then_0
      (bind _returnvalue (Game|ConstructObjectfromClass "/Game/Blueprints/BP_CheckerboardController.BP_CheckerboardController_C" Playground))
      (Variables|/Game/Blueprints/BP_GamePlayground.BP_GamePlayground_C|SetController Playground _returnvalue))
    (:then_1
      (Default|InitPlayer Playground))
    (:then_2
      (bind _modalwidget (Default|CreateInfoModal Playground))
      (bind _output_get (Variables|Default|SetModal%20Widget _modalwidget))
      (Default|SetInfoText _output_get (Utilities|Text|FormatText "游戏开始")))
    (:then_3
      (Variables|/Game/Blueprints/BP_GamePlayground.BP_GamePlayground_C|SetCurrentRound Playground 0))))

(fn OnEndGameStage
  (params (Playground :type BP%20Game%20Playground%20Object%20Reference) (NextStage :type Enum_GameStage%20Enum :default "NewEnumerator7"))
  (|CallParentFunction 0 "NewEnumerator0"))