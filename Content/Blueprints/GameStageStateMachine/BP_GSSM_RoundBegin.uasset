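; BP_GSSM_RoundBegin is the game stage state that opens each round on the playground.
; On entering, it calls the parent, initializes the checkerboard, increments the round counter, shows the round number in an info modal and moves the camera to the playground's focus point.
; An execute-interact interface event closes the modal and advances the playground to another game stage.
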(event EventBPIExecuteInteract
  (params (GamePlayerground :type BP%20Game%20Playground%20Object%20Reference) (Controller :type Checkerboard%20Controller%20Object%20Reference))
  (Class|ModalWidget|Close (Variables|Default|GetModal%20Widget))
  (Default|SetGameStage GamePlayerground "NewEnumerator4"))

(fn OnBeginGameStage
  (params (Playground :type BP%20Game%20Playground%20Object%20Reference) (PrevStage :type Enum_GameStage%20Enum :default "NewEnumerator7"))
  (|CallParentFunction Playground PrevStage)
  (Utilities|FlowControl|Sequence
    (:then_0
      (Default|InitCheckerboard Playground))
    (:then_1
      ;[1 1 1] 回合计数+1
      (Variables|/Game/Blueprints/BP_GamePlayground.BP_GamePlayground_C|SetCurrentRound Playground (+ (Variables|/Game/Blueprints/BP_GamePlayground.BP_GamePlayground_C|GetCurrentRound Playground) 1)))
    (:then_2
      ;[1 1 1] 展示回合信息
      (bind _modalwidget (Default|CreateInfoModal Playground))
      (bind _output_get (Variables|Default|SetModal%20Widget _modalwidget))
      (Default|SetInfoText _output_get (Utilities|Text|FormatText "第 {0} 回合 " (Variables|/Game/Blueprints/BP_GamePlayground.BP_GamePlayground_C|GetCurrentRound Playground))))
    (:then_3
      (Default|MoveCameratoFocusPoint Playground (Variables|/Game/Blueprints/BP_GamePlayground.BP_GamePlayground_C|GetFocusGlobalTransform Playground)))))