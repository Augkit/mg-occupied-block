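; BP_GSSM_TurnBegin is the game-stage state that opens each player's turn in a tetromino puzzle placement game.
; On stage begin it calls the parent, advances the playground to the next player, shows an info modal naming that player, then deals tetrominos.
; The interface execute-interact event closes the stored modal and switches the playground to another game stage.
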(event EventBPIExecuteInteract
  (params (GamePlayerground :type BP%20Game%20Playground%20Object%20Reference) (Controller :type Checkerboard%20Controller%20Object%20Reference))
  (Class|ModalWidget|Close (Variables|Default|GetModal%20Widget))
  (Default|SetGameStage GamePlayerground "NewEnumerator0"))

(fn OnBeginGameStage
  (params (Playground :type BP%20Game%20Playground%20Object%20Reference) (PrevStage :type Enum_GameStage%20Enum :default "NewEnumerator7"))
  (|CallParentFunction Playground PrevStage)
  (Default|NextPlayer Playground)
  (bind _modalwidget (Default|CreateInfoModal Playground))
  (bind _output_get (Variables|Default|SetModal%20Widget _modalwidget))
  (Default|SetInfoText _output_get (Utilities|Text|FormatText "轮到 {0} 放置拼图" (.Name (Utilities|Struct|BreakStru_PlayerInfo (Utilities|Array|Get(acopy) (Variables|/Game/Blueprints/BP_GamePlayground.BP_GamePlayground_C|GetPlayerInfos Playground) (Variables|/Game/Blueprints/BP_GamePlayground.BP_GamePlayground_C|GetCurrentPlayerIndex Playground))))))
  (Default|DealTetrominos Playground))