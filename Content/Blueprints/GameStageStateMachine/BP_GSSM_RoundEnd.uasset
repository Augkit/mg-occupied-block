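; Round-end state of the game stage state machine, which settles the round winner and decides whether the game continues.
; On begin it updates the scoreboard, then either switches stage if someone has won the game or shows a modal naming the round winner.
; The interact event closes the modal and advances the stage.
; Checkerboard and player state cleanup waits until stage end so the winner can be calculated first.
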(event EventBPIExecuteInteract
  (params (GamePlayerground :type BP%20Game%20Playground%20Object%20Reference) (Controller :type Checkerboard%20Controller%20Object%20Reference))
  (Class|ModalWidget|Close (Variables|Default|GetModal%20Widget))
  (Default|SetGameStage GamePlayerground "NewEnumerator5"))

(fn OnBeginGameStage
  (params (Playground :type BP%20Game%20Playground%20Object%20Reference) (PrevStage :type Enum_GameStage%20Enum :default "NewEnumerator7"))
  (|CallParentFunction Playground PrevStage)
  (Utilities|FlowControl|Sequence
    (:then_0
      (bind _winnerindex (Default|CalcThisRoundWinner Playground))
      (bind _output_get (Variables|Default|SetWinner%20Index _winnerindex))
      (Default|UpdatePlayerScoreboard Playground _output_get))
    (:then_1
      (if (.HasGameWinner (Default|WhoWinThisGame Playground))
        (Default|SetGameStage Playground "NewEnumerator9")
        (else
          (bind _modalwidget (Default|CreateInfoModal Playground))
          (bind _output_get_2 (Variables|Default|SetModal%20Widget _modalwidget))
          (Default|SetInfoText _output_get_2 (Utilities|Text|FormatText "{0} 获得了本轮胜利" (.Name (Utilities|Struct|BreakStru_PlayerInfo (Utilities|Array|Get(acopy) (Variables|/Game/Blueprints/BP_GamePlayground.BP_GamePlayground_C|GetPlayerInfos Playground) (Variables|Default|GetWinner%20Index)))))))))))

(fn OnEndGameStage
  (params (Playground :type BP%20Game%20Playground%20Object%20Reference) (NextStage :type Enum_GameStage%20Enum :default "NewEnumerator7"))
  (|CallParentFunction Playground NextStage)
  ;[1 1 1] 清理这一轮的数据，没有在OnBegin中清理是为了计算本轮胜利者
  (Default|DestroyCheckerboard Playground)
  (Default|ResetPlayerState Playground))