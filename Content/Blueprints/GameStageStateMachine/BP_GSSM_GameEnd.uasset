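; Game-stage state for the end of a match in the game stage state machine, announcing the winner.
; On begin, it opens a transition modal from the Playground and shows a Chinese victory message with the winning player's name.
; The interact interface event closes the modal, and a close handler, presumably bound to the modal's close callback, switches the Playground to another game stage.
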(event EventBPIExecuteInteract
  (params (GamePlayerground :type BP%20Game%20Playground%20Object%20Reference) (Controller :type Checkerboard%20Controller%20Object%20Reference))
  (bind _modal_widget (Variables|Default|GetModal%20Widget)
    (:then
      (Class|ModalWidget|Close _modal_widget))
    (:else)))

(fn OnBeginGameStage
  (params (Playground :type BP%20Game%20Playground%20Object%20Reference) (PrevStage :type Enum_GameStage%20Enum :default "NewEnumerator7"))
  (|CallParentFunction Playground PrevStage)
  (Variables|Default|SetPlayground Playground)
  (bind _modalwidget (Default|CreateTransitionModal Playground))
  (bind _output_get (Variables|Default|SetModal%20Widget _modalwidget))
  (Default|SetInfoText _output_get (Utilities|Text|FormatText "获得游戏胜利的是 {0} ！！！" (.Name (Utilities|Struct|BreakStru_PlayerInfo (Utilities|Array|Get(acopy) (Variables|/Game/Blueprints/BP_GamePlayground.BP_GamePlayground_C|GetPlayerInfos Playground) (.PlayerIndex (Default|WhoWinThisGame Playground)))))))
  (EventDispatchers|BindEventtoOnCloseModal _output_get (EventDispatchers|CreateEvent :!event HandleCloseTransition)))

(fn OnEndGameStage
  (params (Playground :type BP%20Game%20Playground%20Object%20Reference) (NextStage :type Enum_GameStage%20Enum :default "NewEnumerator7"))
  (|CallParentFunction Playground NextStage))

(fn HandleCloseTransition
  (Default|SetGameStage (Variables|Default|GetPlayground) "NewEnumerator7"))