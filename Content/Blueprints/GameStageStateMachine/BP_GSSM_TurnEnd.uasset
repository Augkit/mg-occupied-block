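; Turn-end stage of the game stage state machine, which wraps up the current player's turn in a tetromino puzzle game.
; On entering the stage, it updates the current player's scoreboard, then destroys every tetromino left in the hand.
; It then sets the next stage on the Playground: game over if only one player survives, otherwise the next turn.
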(fn OnBeginGameStage
  (params (Playground :type BP%20Game%20Playground%20Object%20Reference) (PrevStage :type Enum_GameStage%20Enum :default "NewEnumerator7"))
  (|CallParentFunction Playground PrevStage)
  (Utilities|FlowControl|Sequence
    (:then_0
      ;[1 1 1] 更新计分板
      (Default|UpdatePlayerScoreboard Playground (Variables|/Game/Blueprints/BP_GamePlayground.BP_GamePlayground_C|GetCurrentPlayerIndex Playground)))
    (:then_1
      ;[1 1 1] 清理拼图块
      (while (> (Utilities|Array|Length (Variables|/Game/Blueprints/BP_GamePlayground.BP_GamePlayground_C|GetHandTetrominos Playground)) 0)
        (Default|DestroyTetromino Playground (Utilities|Array|Get(acopy) (Variables|/Game/Blueprints/BP_GamePlayground.BP_GamePlayground_C|GetHandTetrominos Playground)))))
    (:then_2
      (if (Default|IsOnlyOnePlayerSurvives Playground)
        ;[1 1 1] 如果当前玩家投降则本局游戏结束
        (Default|SetGameStage Playground "NewEnumerator6")
        (else
          ;[1 1 1] 进入下一回合
          (Default|SetGameStage Playground "NewEnumerator4"))))))