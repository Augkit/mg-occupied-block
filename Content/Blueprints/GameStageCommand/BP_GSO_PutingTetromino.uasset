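; Game stage command Blueprint that handles player input while a tetromino is being placed on the board.
; It overrides the interact, four directional move and rotate commands, calling the parent version first in each.
; Each override then forwards to the matching GamePlayerground function to move, rotate or put the tetromino onto the board.
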(fn ExecuteInteract
  (params (GamePlayerground :type BP%20Game%20Playground%20Object%20Reference) (Controller :type Checkerboard%20Controller%20Object%20Reference))
  (|CallParentFunction GamePlayerground Controller)
  (Default|PutTetrominotoBoard GamePlayerground))

(fn ExecuteMoveUp
  (params (GamePlayerground :type BP%20Game%20Playground%20Object%20Reference) (Controller :type Checkerboard%20Controller%20Object%20Reference))
  (|CallParentFunction GamePlayerground Controller)
  (Default|MoveTetrominoUp GamePlayerground))

(fn ExecuteMoveDown
  (params (GamePlayerground :type BP%20Game%20Playground%20Object%20Reference) (Controller :type Checkerboard%20Controller%20Object%20Reference))
  (|CallParentFunction GamePlayerground Controller)
  (Default|MoveTetrominoDown GamePlayerground))

(fn ExecuteMoveRight
  (params (GamePlayerground :type BP%20Game%20Playground%20Object%20Reference) (Controller :type Checkerboard%20Controller%20Object%20Reference))
  (|CallParentFunction GamePlayerground Controller)
  (Default|MoveTetrominoRight GamePlayerground))

(fn ExecuteMoveLeft
  (params (GamePlayerground :type BP%20Game%20Playground%20Object%20Reference) (Controller :type Checkerboard%20Controller%20Object%20Reference))
  (|CallParentFunction GamePlayerground Controller)
  (Default|MoveTetrominoLeft GamePlayerground))

(fn ExexuteRotate
  (params (GamePlayerground :type BP%20Game%20Playground%20Object%20Reference) (Controller :type Checkerboard%20Controller%20Object%20Reference))
  (|CallParentFunction GamePlayerground Controller)
  (Default|RotateTetromino GamePlayerground))